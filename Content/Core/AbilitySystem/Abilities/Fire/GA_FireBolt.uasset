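; Fire Bolt gameplay ability that casts a projectile toward the point under the mouse.
; On activation, a target data task supplies the hit point, and the avatar turns toward it through the Aura combat interface.
; It plays the cast montage and waits for its Firebolt gameplay event to time the inherited SpawnProjectile call.
; The ability ends after a short delay following the spawn.
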(event Ability|EventActivateAbility
  (bind _datahandle (|TargetDataUnderMouse)
    (:ValidDataDelegate
      (Variables|Default|SetProjectileTargetLocation (.ImpactPoint (Collision|BreakHitResult (Ability|TargetData|GetHitResultfromTargetData _datahandle))))
      (bind _asaura_combat_interface (Utilities|Casting|CastToAuraCombatInterface (Ability|GetAvatarActorfromActorInfo)))
      (Class|AuraCombatInterface|SetFacingTarget _asaura_combat_interface (Variables|Default|GetProjectileTargetLocation))
      (|PlayMontageandWaitProxy "None" "/Game/Assets/Characters/Aura/Animations/Abilities/AM_CastFirebolt.AM_CastFirebolt" 1.0 "None" true 1.0 0.0 false
        (:then
          (Ability|Tasks|WaitGameplayEvent "(TagName=\"Event.Montage.Firebolt\")" 0
            (:EventReceived
              (Class|AuraFireBolt|SpawnProjectile (Variables|Default|GetProjectileTargetLocation))
              (Utilities|FlowControl|Delay 0.5)
              (Ability|EndAbility))))))))

(event Ability|EventOnEndAbility
  (params (bWasCancelled :type Boolean)))